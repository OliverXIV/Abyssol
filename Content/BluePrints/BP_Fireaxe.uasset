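; BP_Fireaxe is a fire axe actor, commented as a collectible that highlights while the camera looks at it.
; Tick turns on custom depth for its child meshes and sets Allow1Interaction, with no camera test.
; Chained Delays and three one-shot flags clear highlight and interaction on early passes, then destroy the actor as "collected" once all are set.
; The Interacting event is empty, so Tick alone drives this sequence.
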(event `/Game/BluePrints/FP_Interaction.Interacting`
  (params (Camera :type "Actor Object Reference"))
  ;[0.05035 0.05035 0.05035] Camera Looking At Object
)

(event `self.ReceiveTick`
  (params (DeltaSeconds :type "Float (single-precision)"))
  ;[0.05035 0.05035 0.05035] Camera Looking At Object
  (for _array_element (`SceneComponent.GetChildrenComponents` (`self.DefaultSceneRoot`) false)
    (bind _asmesh_component (cast `MeshComponent` _array_element))
    (`PrimitiveComponent.SetRenderCustomDepth` _asmesh_component true))
  (set `self.Allow1Interaction` true)
  (`KismetSystemLibrary.Delay` 0.15)
  (if (`self.FirstCheck`)
    (`KismetSystemLibrary.Delay` 0.15)
    (if (`self.SecondCheck`)
      (`KismetSystemLibrary.Delay` 0.15)
      (if (`self.ThirdCheck`)
        ;[1 1 1] Collected Item
        (`self.K2_DestroyActor`)
        (else
          (set `self.ThirdCheck` true)
          ;[1 1 1] Camera Stopped Looking At Axe
          (for _array_element_2 (`SceneComponent.GetChildrenComponents` (`self.DefaultSceneRoot`) false) :!label _label
            (bind _asmesh_component_2 (cast `MeshComponent` _array_element_2))
            (`PrimitiveComponent.SetRenderCustomDepth` _asmesh_component_2 false))
          (set `self.Allow1Interaction` false)))
      (else
        (set `self.SecondCheck` true)
        (goto _label)))
    (else
      (set `self.FirstCheck` true)
      (goto _label))))

(fn `UserConstructionScript`)