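; Tutorial cabinet that opens once on actor overlap to present a case file to the player.
; The drawer eases out, a placeholder case file hops up and down, then a case file actor flagged as Tutorial spawns at its transform.
; If untouched ten seconds after BeginPlay, a question mark appears and bobs until the interaction, which hides it.
; A Test flag fires the opening sequence at BeginPlay.
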(event `self.ReceiveActorBeginOverlap`
  (params (OtherActor :type "Actor Object Reference"))
  (bind _bp_testinteractiocasefileforposechangecolor (`self.BP_TestInteractioCasefileForPoseChangeColor`))
  (bind _drawer (`self.Drawer`))
  (bind _relativelocation (`SceneComponent.RelativeLocation` _bp_testinteractiocasefileforposechangecolor))
  (bind _relativerotation (`SceneComponent.RelativeRotation` _bp_testinteractiocasefileforposechangecolor))
  (if (not (`self.InteractedYOHOU`)) :!label _label
    (set `self.InteractedYOHOU` true)
    (`KismetSystemLibrary.MoveComponentTo` (`self.Drawer`) (+ (`SceneComponent.RelativeLocation` _drawer) (0.0 60.0 0.0)) (`SceneComponent.RelativeRotation` _drawer) true false 1.0)
    (`SceneComponent.ToggleVisibility` _bp_testinteractiocasefileforposechangecolor false)
    (`KismetSystemLibrary.MoveComponentTo` _bp_testinteractiocasefileforposechangecolor (+ _relativelocation (0.0 0.0 25.0)) _relativerotation true false 0.3)
    (`KismetSystemLibrary.MoveComponentTo` _bp_testinteractiocasefileforposechangecolor (+ _relativelocation (0.0 0.0 -25.0)) _relativerotation false true 0.3)
    (`SceneComponent.ToggleVisibility` _bp_testinteractiocasefileforposechangecolor false)
    (bind _returnvalue (`|SpawnActorFromClass` "/Game/BluePrints/BP_TestInteractioCasefileForPoseChangeColor.BP_TestInteractioCasefileForPoseChangeColor_C" (`SceneComponent.K2_GetComponentToWorld` (`self.BP_TestInteractioCasefileForPoseChangeColor`)) "Undefined" "MultiplyWithRoot" null null))
    (set `/Game/BluePrints/BP_TestInteractioCasefileForPoseChangeColor.Tutorial?` true _returnvalue)
    (`SceneComponent.SetVisibility` (`self.S_Question_Mark`) false false)))

(event `self.ReceiveBeginPlay`
  (bind _interactedyohou (`self.InteractedYOHOU`))
  (bind _relativerotation (`SceneComponent.RelativeRotation` (`self.S_Question_Mark`)))
  (`|ExecutionSequence`
    (:`then_0`
      (`KismetSystemLibrary.Delay` 10.0)
      (if (not _interactedyohou)
        (`SceneComponent.SetVisibility` (`self.S_Question_Mark`) true false)
        (if (not _interactedyohou) :!label _label_2
          (`KismetSystemLibrary.MoveComponentTo` (`self.S_Question_Mark`) (0.0 0.0 130.0) _relativerotation true true 1.0)
          (`KismetSystemLibrary.MoveComponentTo` (`self.S_Question_Mark`) (0.0 0.0 110.0) _relativerotation true true 1.0)
          (goto _label_2))))
    (:`then_1`
      (if (`self.Test`)
        (goto _label)))))

(fn `UserConstructionScript`)