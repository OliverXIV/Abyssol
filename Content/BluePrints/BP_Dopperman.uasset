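; BP_Dopperman is a dialogue Blueprint that steps through an array of welcome and story explanation lines in a WB_Dialogue widget.
; BeginPlay (if 1stAutomatic), a Tick Delay acting as a repeating timer (if AutomaticPlay), and StartGameByPressingButton share one advance routine.
; That routine lazily creates the widget for player controller index 1, shows the next line, then removes it and sets DialogueFinished once lines run out.
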(event `self.ReceiveBeginPlay`
  (bind _welcome_dialogue___story_explainations (`self.Welcome Dialogue + Story Explainations`))
  (bind _talkindex (`self.TalkIndex`))
  (if (`self.1stAutomatic`)
    (if (< _talkindex (`KismetArrayLibrary.Array_Length` _welcome_dialogue___story_explainations)) :!label _label
      (`self.UI`
        (:`then`
          _)
        (:`else`
          (bind _returnvalue (`|CreateWidget` "/Game/BluePrints/WB_Dialogue.WB_Dialogue_C" (`GameplayStatics.GetPlayerController` 1)))
          (bind _output_get (set `self.UI` _returnvalue))
          (`UserWidget.AddToViewport` _output_get 0)))
      (`TextBlock.SetText` (`/Game/BluePrints/WB_Dialogue.TalkText` (`self.UI`)) (`KismetTextLibrary.Conv_StringToText` (`|GetArrayItem` _welcome_dialogue___story_explainations _talkindex)))
      (`/Engine/EditorBlueprintResources/StandardMacros.IncrementInt` (`self.TalkIndex`))
      (else
        (`Widget.RemoveFromParent` (`self.UI`))
        (set `self.DialogueFinished` true)))))

(event `self.ReceiveTick`
  (params (DeltaSeconds :type "Float (single-precision)"))
  (`KismetSystemLibrary.Delay` 3.0)
  (if (`self.AutomaticPlay`)
    (goto _label)))

(event `StartGameByPressingButton`
  (goto _label))

(fn `UserConstructionScript`)