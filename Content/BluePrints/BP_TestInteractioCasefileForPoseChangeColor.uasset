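; Inspectable case file prop that moves up to the camera to show its text and returns to its saved transform when dismissed.
; Interacting briefly enables custom depth highlighting and opens the window for TriggerInspect to start viewing.
; While viewed, a per-tick MoveComponentTo loop tracks the camera.
; In tutorial mode, an untouched file shows a bobbing question mark, and dismissing it triggers BP_Dopperman dialogue and destroys the actor.
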(event `/Game/BluePrints/FP_Interaction.Interacting`
  (params (Camera :type "Actor Object Reference"))
  ;[0.05035 0.05035 0.05035] Camera Looking At Object
  (for _array_element (`SceneComponent.GetChildrenComponents` (`self.DefaultSceneRoot`) false)
    (bind _asmesh_component (cast `MeshComponent` _array_element))
    (`PrimitiveComponent.SetRenderCustomDepth` _asmesh_component true))
  (set `self.Allow1Interaction` true)
  (`KismetSystemLibrary.RetriggerableDelay` 0.15)
  (for _array_element_2 (`SceneComponent.GetChildrenComponents` (`self.DefaultSceneRoot`) false)
    (bind _asmesh_component_2 (cast `MeshComponent` _array_element_2))
    (`PrimitiveComponent.SetRenderCustomDepth` _asmesh_component_2 false))
  (set `self.Allow1Interaction` false))

(event `TriggerInspect`
  (bind _viewobject (`self.ViewObject`))
  ;[0.05035 0.05035 0.05035] Zoom On Object Interaction
  (if (`self.Allow1Interaction`) :!label _label
    (if (not _viewobject)
      (set `self.ViewObject` true)
      (set `self.Interacted YOO` true)
      (`SceneComponent.SetVisibility` (`self.S_Question_Mark`) false false)
      (`SceneComponent.SetVisibility` (`self.TextRender`) true false)
      (bind (_returnvalue_roll _returnvalue_pitch _returnvalue_yaw) (`KismetMathLibrary.BreakRotator` (`self.K2_GetActorRotation` (stale `/Game/BluePrints/FP_Interaction.Interacting` Camera))))
      (`KismetSystemLibrary.MoveComponentTo` (`self.DefaultSceneRoot`) (+ (`self.K2_GetActorLocation` (stale `/Game/BluePrints/FP_Interaction.Interacting` Camera)) (100.0 0.0 -5.0)) (`KismetMathLibrary.MakeRotator` _returnvalue_roll (+ _returnvalue_pitch (`self.PitchRotationAdd`)) (+ _returnvalue_yaw 180.0)) true false 0.5 true :!label _label_2)
      (if (`self.ViewObject`)
        (`KismetSystemLibrary.DelayUntilNextTick`)
        (goto _label_2)))
    (elif _viewobject
      (set `self.ViewObject` false)
      (set `self.Interacted YOO` true)
      (if (`self.Tutorial?`)
        (bind _outactors (`GameplayStatics.GetAllActorsOfClass` "/Game/BluePrints/BP_Dopperman.BP_Dopperman_C"))
        (for _array_element _outactors
          (set `/Game/BluePrints/BP_Dopperman.Dialogue Time` true _array_element))
        (`self.K2_DestroyActor`)
        (else
          (`SceneComponent.SetVisibility` (`self.TextRender`) false false)
          (`KismetSystemLibrary.MoveComponentTo` (`self.DefaultSceneRoot`) (`self.SaveLocation`) (`self.SaveRotation`) true false 0.5 true))))))

(event `self.ReceiveTick`
  (params (DeltaSeconds :type "Float (single-precision)"))
  ;[0.05035 0.05035 0.05035] Zoom On Object Interaction
  (if (`self.TestInteraction`)
    (`KismetSystemLibrary.Delay` 3.0)
    (goto _label)))

(event `self.ReceiveBeginPlay`
  (bind _s_question_mark (`self.S_Question_Mark`))
  (bind _interacted_yoo (`self.Interacted YOO`))
  (bind _s_question_mark_2 (`self.S_Question_Mark`))
  (bind _relativerotation (`SceneComponent.RelativeRotation` _s_question_mark))
  (bind _relativelocation (`SceneComponent.RelativeLocation` _s_question_mark))
  ;[0.05035 0.05035 0.05035] Zoom On Object Interaction
  (set `self.SaveLocation` (`SceneComponent.K2_GetComponentLocation` (`self.DefaultSceneRoot`)))
  (set `self.SaveRotation` (`SceneComponent.K2_GetComponentRotation` (`self.DefaultSceneRoot`)))
  (`KismetSystemLibrary.Delay` 0.2)
  (if (`self.Tutorial?`)
    (`KismetSystemLibrary.Delay` 10.0)
    (if (not _interacted_yoo)
      (`SceneComponent.SetVisibility` _s_question_mark_2 true false)
      (if (not _interacted_yoo) :!label _label_3
        (`KismetSystemLibrary.MoveComponentTo` _s_question_mark_2 (+ _relativelocation (0.0 0.0 20.0)) _relativerotation true true 1.0)
        (`KismetSystemLibrary.MoveComponentTo` _s_question_mark_2 (+ _relativelocation (0.0 0.0 -20.0)) _relativerotation true true 1.0)
        (goto _label_3)))))

(fn `UserConstructionScript`)